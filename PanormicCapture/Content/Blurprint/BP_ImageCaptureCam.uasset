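; BP_ImageCaptureCam is a camera actor that captures left and right images to render targets through two scene capture components.
; The construction script treats the Capture bool as a one-shot button, triggering both captures, resetting itself and printing a confirmation.
; It then applies SizeX to both render targets and CaptureSource to both components, so these changes follow that run's capture.
; The event graph is empty.
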(event EventBeginPlay)

(event Collision|EventActorBeginOverlap
  (params (OtherActor :type Actor%20Object%20Reference)))

(event EventTick
  (params (DeltaSeconds :type Float%20%28single-precision%29)))

(fn ConstructionScript
  (Utilities|FlowControl|Sequence
    (:then_0
      (if (Variables|Default|GetCapture)
        (Rendering|SceneCapture|CaptureScene (Variables|Default|GetSceneCapture_L) :!class /Script/Engine.SceneCaptureComponentCube)
        (Rendering|SceneCapture|CaptureScene (Variables|Default|GetSceneCapture_R) :!class /Script/Engine.SceneCaptureComponentCube)
        (Variables|Default|SetCapture false)
        (Development|PrintString "Captured")))
    (:then_1
      (Variables|/Script/Engine.TextureRenderTargetCube|SetSizeX (Variables|/Script/Engine.SceneCaptureComponentCube|GetTextureTarget (Variables|Default|GetSceneCapture_L)) (Variables|Default|GetSize%20X))
      (Variables|/Script/Engine.TextureRenderTargetCube|SetSizeX (Variables|/Script/Engine.SceneCaptureComponentCube|GetTextureTarget (Variables|Default|GetSceneCapture_R)) (Variables|Default|GetSize%20X)))
    (:then_2
      (Variables|/Script/Engine.SceneCaptureComponent|SetCaptureSource (Variables|Default|GetSceneCapture_L) (Variables|Default|GetCapture%20Source))
      (Variables|/Script/Engine.SceneCaptureComponent|SetCaptureSource (Variables|Default|GetSceneCapture_R) (Variables|Default|GetCapture%20Source)))))