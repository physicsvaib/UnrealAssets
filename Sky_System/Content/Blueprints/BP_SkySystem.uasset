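; Sky system actor that sets sun, moon, atmosphere, stars and clouds from a time-of-day value.
; Construction script creates dynamic sky sphere and volumetric cloud materials, then applies all settings; nothing runs on Tick.
; Dawn and dusk drive light rotation, visibility and sun temperature, and switch night scattering scale and stars.
; Cloud mode selects none, 2D clouds in the sky material, or 3D volumetric clouds.
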(event EventBeginPlay)

(event Collision|EventActorBeginOverlap
  (params (OtherActor :type Actor%20Object%20Reference)))

(event EventTick
  (params (DeltaSeconds :type Float%20%28single-precision%29)))

(fn ConstructionScript
  (01-BasicSettings|CreateMaterialInstance)
  (01-BasicSettings|UpdateBasicInfo))

(fn CreateMaterialInstance
  (Utilities|FlowControl|Sequence
    (:then_0
      (Utilities|IsValid (Variables|01-BasicSettings|GetStarMaterial)
        (:Is%20Not%20Valid
          (bind _returnvalue (Rendering|Material|CreateDynamicMaterialInstance "/Sky_System/Materials/SkySphere/MI_SkySphere.MI_SkySphere" "None" "None" :!class /Script/Engine.KismetMaterialLibrary))
          (bind _output_get (Variables|01-BasicSettings|SetStarMaterial _returnvalue))
          (Rendering|Material|SetMaterial (Variables|Default|GetSkySphere) 0 _output_get))))
    (:then_1
      (Utilities|IsValid (Variables|03-Clouds|Get3D%20Cloud%20Mat)
        (:Is%20Not%20Valid
          (bind _returnvalue_2 (Rendering|Material|CreateDynamicMaterialInstance "/Sky_System/Materials/VolumetricCloud/MI_Clouds.MI_Clouds" "None" "None" :!class /Script/Engine.KismetMaterialLibrary))
          (bind _output_get_2 (Variables|03-Clouds|Set3D%20Cloud%20Mat _returnvalue_2))
          (Rendering|Material|SetMaterial (Variables|Default|GetVolumetricCloud) _output_get_2))))))

(fn HandleSunRotation
  (bind _timeofday (Variables|01-BasicSettings|GetTImeOfDay))
  (bind _dawntime (Variables|01-BasicSettings|GetDawnTime))
  (bind _returnvalue (+ _dawntime -0.3))
  (Transformation|SetWorldRotation (Variables|Default|GetSunLight) (Math|Rotator|MakeRotator 0.0 (Math|Float|MapRangeUnclamped (Variables|01-BasicSettings|GetTImeOfDay) (Variables|01-BasicSettings|GetDawnTime) (Variables|01-BasicSettings|GetDuskTime) 0.0 -1.8e+02) 0.0) false false)
  (Transformation|SetWorldRotation (Variables|Default|GetMoonLight) (Math|Rotator|MakeRotator 0.0 (Math|Float|SelectFloat (Math|Float|MapRangeUnclamped _timeofday 0.0 _returnvalue -9e+01 -1.8e+02) (Math|Float|MapRangeUnclamped _timeofday (+ (Variables|01-BasicSettings|GetDuskTime) 0.3) 24.0 0.0 -9e+01) (< _timeofday _returnvalue)) 0.0) false false))

(fn HandleVisibilty
  (bind _isday (Utilities|IsDayTime))
  (Rendering|SetVisibility (Variables|Default|GetSunLight) _isday false)
  (Rendering|SetVisibility (Variables|Default|GetMoonLight) (not _isday) false))

(fn UpdateBasicInfo
  (Utilities|IsValid (Variables|01-BasicSettings|GetStarMaterial)
    (:Is%20Valid
      (Utilities|FlowControl|Sequence
        (:then_1
          (01-BasicSettings|HandleSunRotation))
        (:then_2
          (01-BasicSettings|HandleVisibilty))
        (:then_3
          (02-NightSettings|ToggleNightSettings))
        (:then_4
          (01-BasicSettings|HandleTemprature))
        (:then_5
          (03-Clouds|HandleCloudSettings))))
    (:Is%20Not%20Valid
      (Development|PrintString "Failed to Init Material Instance"))))

(fn ToggleNightSettings
  (bind _skyatmosphere (Variables|Default|GetSkyAtmosphere))
  (bind _skyatmosphere_2 (Variables|Default|GetSkyAtmosphere))
  (if (Utilities|IsDayTime)
    (Class|SkyAtmosphereComponent|SetRayleighScattering _skyatmosphere (Variables|02-NightSettings|GetNightLightScatter))
    (Class|SkyAtmosphereComponent|SetRayleighScatteringScale _skyatmosphere (Variables|02-NightSettings|GetDayRayLeigh))
    ;[1 1 1] Remove these if you want to control stars on your own
    (02-NightSettings|SetStarsStatus false)
    (else
      (Class|SkyAtmosphereComponent|SetRayleighScattering _skyatmosphere_2 (Variables|02-NightSettings|GetNightLightScatter))
      (Class|SkyAtmosphereComponent|SetRayleighScatteringScale _skyatmosphere_2 (Variables|02-NightSettings|GetNightRayLeigh))
      (02-NightSettings|SetStarsStatus true))))

(fn HandleTemprature
  (bind _returnvalue (Utilities|HalfTime))
  (bind _timeofday (Variables|01-BasicSettings|GetTImeOfDay))
  (Class|LightComponent|SetTemperature (Variables|Default|GetSunLight) (Math|Float|SelectFloat (Math|Float|MapRangeUnclamped _timeofday _returnvalue (Variables|01-BasicSettings|GetDuskTime) 4e+03 6e+03) (Math|Float|MapRangeUnclamped (Variables|01-BasicSettings|GetTImeOfDay) (Variables|01-BasicSettings|GetDawnTime) _returnvalue 6e+03 4e+03) (> _timeofday _returnvalue))))

(fn SetStarsStatus
  (params (Visible :type Boolean))
  (Rendering|Material|SetScalarParameterValue (Variables|01-BasicSettings|GetStarMaterial) "ShouldStarsBePresent" (Math|Float|SelectFloat 1.0 0.0 Visible) :!class /Script/Engine.MaterialInstanceDynamic))

(fn HandleCloudSettings
  (bind _starmaterial (Variables|01-BasicSettings|GetStarMaterial))
  (switch Utilities|FlowControl|Switch|SwitchonE_CloudMode (Variables|03-Clouds|GetCurrentCloudMode)
    (:NewEnumerator0
      (Utilities|FlowControl|Sequence
        (:then_0
          (Rendering|SetVisibility (Variables|Default|GetVolumetricCloud) false false :!label _label))
        (:then_1
          (Rendering|Material|SetScalarParameterValue _starmaterial "ShouldCloudsBePresent" 0.0 :!class /Script/Engine.MaterialInstanceDynamic :!label _label_2))))
    (:NewEnumerator1
      (Utilities|FlowControl|Sequence
        (:then_0
          (goto _label))
        (:then_1
          (Rendering|Material|SetScalarParameterValue _starmaterial "ShouldCloudsBePresent" 1.0 :!class /Script/Engine.MaterialInstanceDynamic)
          (Rendering|Material|SetVectorParameterValue _starmaterial "CloudSettings" (Utilities|BaseCloudSettings) :!class /Script/Engine.MaterialInstanceDynamic))))
    (:NewEnumerator2
      (Utilities|FlowControl|Sequence
        (:then_0
          (goto _label_2))
        (:then_1
          (Rendering|SetVisibility (Variables|Default|GetVolumetricCloud) true false)
          ;[0.1488 1 0] Check The MI for more options
          (03-Clouds|Init3DCloudSettings))))))

(fn Init3DCloudSettings
  (bind _3d_cloud_mat (Variables|03-Clouds|Get3D%20Cloud%20Mat))
  (bind _3dpanspeed (Variables|03-Clouds|Get3DPanSpeed))
  (bind _volumetriccloud (Variables|Default|GetVolumetricCloud))
  (bind (_x _y) (Math|Vector2D|BreakVector2D _3dpanspeed))
  (Rendering|Material|SetScalarParameterValue _3d_cloud_mat "PanningSpeedX" _x :!class /Script/Engine.MaterialInstanceDynamic)
  (Rendering|Material|SetScalarParameterValue _3d_cloud_mat "PanningSpeedY" _y :!class /Script/Engine.MaterialInstanceDynamic)
  (Class|VolumetricCloudComponent|SetLayerBottomAltitude _volumetriccloud (Variables|03-Clouds|GetCloudBottomAltitude))
  (Class|VolumetricCloudComponent|SetLayerHeight _volumetriccloud (Variables|03-Clouds|GetCloudHeight)))